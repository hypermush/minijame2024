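; BP_MovingTide is a tide actor that endlessly lowers and raises itself between height targets, pausing randomly at each end.
; Looping timers lerp its Z by an accumulating TideProgress, stopping on an exact height match.
; Each lowering first triggers every BP_Spawner to spawn items and enemies; full high tide deletes them.
; Overlapping its Plane makes a BP_TopDownCharacter dump its inventory through DumpInventoryOnDeath.
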(event `StartLowerTide`
  (bind (_returnvalue_x _returnvalue_y _returnvalue_z) (`KismetMathLibrary.BreakVector` (`self.K2_GetActorLocation`)))
  (bind (_startingspot_x _startingspot_y) (`KismetMathLibrary.BreakVector` (`self.StartingSpot`)))
  (set `self.StartingSpot` (`KismetMathLibrary.MakeVector` _startingspot_x _startingspot_y _returnvalue_z))
  (set `self.TideProgress` 0.0)
  (bind _returnvalue (`KismetSystemLibrary.K2_SetTimerDelegate` (delegate `LowerTideTimer`) 0.2 true :!label _label))
  (set `self.TideMovingTimer` _returnvalue)
  (set `self.IsMovingDown` true))

(event `self.ReceiveBeginPlay`
  (set `self.StartingSpot` (`self.K2_GetActorLocation`))
  (goto _label))

(event `LowerTideTimer`
  (bind (_returnvalue_x _returnvalue_y _returnvalue_z) (`KismetMathLibrary.BreakVector` (`self.K2_GetActorLocation`)))
  (bind (_startingspot_x _startingspot_y) (`KismetMathLibrary.BreakVector` (`self.StartingSpot`)))
  (bind _returnvalue_location (`KismetMathLibrary.BreakTransform` (`KismetMathLibrary.TLerp` (`KismetMathLibrary.MakeTransform` (`self.StartingSpot`)) (`KismetMathLibrary.MakeTransform` (`KismetMathLibrary.MakeVector` _startingspot_x _startingspot_y (`self.MinHeightTarget`))) (`self.TideProgress`))))
  (if (`self.ItemsAndEnemiesSpawned`)
    (`self.K2_SetActorLocation` _returnvalue_location)
    (set `self.TideProgress` (+ (`self.TideProgress`) (`self.TideRate`)))
    (if (== _returnvalue_z (`self.MinHeightTarget`))
      (`KismetSystemLibrary.PrintString` "Low TIde?")
      (`KismetSystemLibrary.K2_ClearAndInvalidateTimerHandle` (`self.TideMovingTimer`))
      (set `self.IsMovingDown` false)
      (`KismetSystemLibrary.Delay` (`KismetMathLibrary.Conv_IntToDouble` (`KismetMathLibrary.RandomIntegerInRange` 5 10)))
      (`self.StartRaiseTide`))
    (else
      (bind _outactors (`GameplayStatics.GetAllActorsOfClass` "/Game/Enemys/BP_Spawner.BP_Spawner_C"))
      (bind _output_get (set `self.Spawners` _outactors))
      (for _array_element _output_get
        (`/Game/Enemys/BP_Spawner.SpawnItemsAndEnemys` _array_element))
      (set `self.ItemsAndEnemiesSpawned` true))))

(event `StartRaiseTide`
  (bind (_returnvalue_x _returnvalue_y _returnvalue_z) (`KismetMathLibrary.BreakVector` (`self.K2_GetActorLocation`)))
  (bind (_startingspot_x _startingspot_y) (`KismetMathLibrary.BreakVector` (`self.StartingSpot`)))
  (set `self.StartingSpot` (`KismetMathLibrary.MakeVector` _startingspot_x _startingspot_y _returnvalue_z))
  (set `self.TideProgress` 0.0)
  (bind _returnvalue (`KismetSystemLibrary.K2_SetTimerDelegate` (delegate `RaiseTideEvent`) 0.2 true))
  (set `self.TideMovingTimer` _returnvalue))

(event `RaiseTideEvent`
  (bind (_returnvalue_x _returnvalue_y _returnvalue_z) (`KismetMathLibrary.BreakVector` (`self.K2_GetActorLocation`)))
  (bind (_startingspot_x _startingspot_y) (`KismetMathLibrary.BreakVector` (`self.StartingSpot`)))
  (bind _returnvalue_location (`KismetMathLibrary.BreakTransform` (`KismetMathLibrary.TLerp` (`KismetMathLibrary.MakeTransform` (`self.StartingSpot`)) (`KismetMathLibrary.MakeTransform` (`KismetMathLibrary.MakeVector` _startingspot_x _startingspot_y (`self.MaxHeightTarget`))) (`self.TideProgress`))))
  (`self.K2_SetActorLocation` _returnvalue_location)
  (set `self.TideProgress` (+ (`self.TideProgress`) (`self.TideRate`)))
  (if (== _returnvalue_z (`self.MaxHeightTarget`))
    (`KismetSystemLibrary.PrintString` "Tide Raised")
    (`KismetSystemLibrary.K2_ClearAndInvalidateTimerHandle` (`self.TideMovingTimer`))
    (for _array_element (`self.Spawners`)
      (`/Game/Enemys/BP_Spawner.DeleteEnemies` _array_element)
      (`/Game/Enemys/BP_Spawner.DeleteItems` _array_element))
    (`KismetSystemLibrary.Delay` (`KismetMathLibrary.Conv_IntToDouble` (`KismetMathLibrary.RandomIntegerInRange` 5 10)))
    (set `self.ItemsAndEnemiesSpawned` false)
    (`self.StartLowerTide`)))

(event `self.Plane.OnComponentBeginOverlap`
  (params (OverlappedComponent :type "PrimitiveComponent Object Reference") (OtherActor :type "Actor Object Reference") (OtherComp :type "PrimitiveComponent Object Reference") (OtherBodyIndex :type Integer) (bFromSweep :type Boolean) (SweepResult :type "HitResult Structure (by ref)"))
  (bind _asbp_top_down_character (cast `/Game/TopDown/Blueprints/BP_TopDownCharacter` OtherActor))
  (`/Game/TopDown/Blueprints/BP_TopDownCharacter.DumpInventoryOnDeath` _asbp_top_down_character))

(fn `UserConstructionScript`)