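; BP_HoardZone is a trigger zone where the top-down player character deposits to the hoard and sees a stats readout.
; On BeginPlay it creates a HoardUI widget, adds it to the viewport and hides it.
; The Cube's begin overlap calls DespoitToHoard on the character, then shows the widget with its Speed, Strength and Progress stats.
; End overlap by any actor hides the widget, without a character check.
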(event `self.ReceiveBeginPlay`
  (bind _returnvalue (`|CreateWidget` "/Game/JoeStuff/UI/HoardUI.HoardUI_C"))
  (bind _output_get (set `self.HoardUIReference` _returnvalue))
  (`UserWidget.AddToViewport` _output_get 0)
  (`Widget.SetVisibility` _output_get "Hidden"))

(event `self.Cube.OnComponentBeginOverlap`
  (params (OverlappedComponent :type "PrimitiveComponent Object Reference") (OtherActor :type "Actor Object Reference") (OtherComp :type "PrimitiveComponent Object Reference") (OtherBodyIndex :type Integer) (bFromSweep :type Boolean) (SweepResult :type "HitResult Structure (by ref)"))
  (bind _hoarduireference (`self.HoardUIReference`))
  (bind _asbp_top_down_character (cast `/Game/TopDown/Blueprints/BP_TopDownCharacter` OtherActor))
  (`/Game/TopDown/Blueprints/BP_TopDownCharacter.DespoitToHoard` _asbp_top_down_character)
  (`Widget.SetVisibility` _hoarduireference "Visible")
  (`TextBlock.SetText` (`/Game/JoeStuff/UI/HoardUI.SpeedCount` _hoarduireference) (`KismetTextLibrary.Conv_IntToText` (`/Game/TopDown/Blueprints/BP_TopDownCharacter.SpeedStat` _asbp_top_down_character)))
  (`TextBlock.SetText` (`/Game/JoeStuff/UI/HoardUI.StrengthCount` _hoarduireference) (`KismetTextLibrary.Conv_IntToText` (`/Game/TopDown/Blueprints/BP_TopDownCharacter.StrengthStat` _asbp_top_down_character)))
  (`TextBlock.SetText` (`/Game/JoeStuff/UI/HoardUI.ProgressCount` _hoarduireference) (`KismetTextLibrary.Conv_IntToText` (`/Game/TopDown/Blueprints/BP_TopDownCharacter.ProgressStat` _asbp_top_down_character))))

(event `self.Cube.OnComponentEndOverlap`
  (params (OverlappedComponent :type "PrimitiveComponent Object Reference") (OtherActor :type "Actor Object Reference") (OtherComp :type "PrimitiveComponent Object Reference") (OtherBodyIndex :type Integer))
  (`Widget.SetVisibility` (`self.HoardUIReference`) "Hidden"))

(fn `UserConstructionScript`)