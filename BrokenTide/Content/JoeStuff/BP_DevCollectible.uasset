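; Developer collectible actor that the player can pick up unless an enemy has grabbed it.
; Overlapping its box with the top-down character sends an interact message.
; Interact checks the IsEnemyGrabbed flag, printing a refusal if set and otherwise calling OnCollect, which destroys the actor.
; Feedback is debug prints only, and nothing in this graph sets the grab flag.
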(event `self.Interact`
  (`KismetSystemLibrary.PrintString` "Interaction!")
  (`self.CheckEnemyGrab`))

(event `self.OnCollect`
  (`self.K2_DestroyActor`))

(event `self.Box.OnComponentBeginOverlap`
  (params (OverlappedComponent :type "PrimitiveComponent Object Reference") (OtherActor :type "Actor Object Reference") (OtherComp :type "PrimitiveComponent Object Reference") (OtherBodyIndex :type Integer) (bFromSweep :type Boolean) (SweepResult :type "HitResult Structure (by ref)"))
  (cast `/Game/TopDown/Blueprints/BP_TopDownCharacter` OtherActor)
  (message `/Game/JoeStuff/CollectibleInterface.Interact` self))

(fn `CheckEnemyGrab`
  (if (`self.IsEnemyGrabbed`)
    (`KismetSystemLibrary.PrintString` "Some other enemy has this!")
    (else
      (`self.OnCollect`))))

(fn `UserConstructionScript`)