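; A collectible pickup that the player can collect or that a crab enemy can grab and carry away.
; A crab overlapping its box attaches it to its hold position and switches to random movement.
; A player overlapping a free item gets an interact message, and interacting destroys it.
; Overlapping a carried item freezes player and crab and starts key-press combat, with key count set by their Strength difference.
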(event `self.Interact`
  (`KismetSystemLibrary.PrintString` "Interaction!")
  (`self.CheckEnemyGrab`))

(event `self.OnCollect`
  (`self.K2_DestroyActor`))

(event `self.Box.OnComponentBeginOverlap`
  (params (OverlappedComponent :type "PrimitiveComponent Object Reference") (OtherActor :type "Actor Object Reference") (OtherComp :type "PrimitiveComponent Object Reference") (OtherBodyIndex :type Integer) (bFromSweep :type Boolean) (SweepResult :type "HitResult Structure (by ref)"))
  (bind _enemyattachedto (`self.EnemyAttachedTo`))
  (bind _asbp_top_down_character (cast `/Game/TopDown/Blueprints/BP_TopDownCharacter` OtherActor)
    (:`then`
      (bind _output_get (set `self.UserForInteraction` _asbp_top_down_character))
      (if (`/Game/TopDown/Blueprints/BP_TopDownCharacter.CombatMode` _output_get)
        _
        (elif (`self.IsEnemyGrabbed`)
          (if (`KismetSystemLibrary.IsValid` _enemyattachedto)
            (`KismetSystemLibrary.K2_ClearAndInvalidateTimerHandle` (`/Game/Enemys/BP_EnemyCrabCharacter.RandomMoveTimer` _enemyattachedto))
            (`CharacterMovementComponent.DisableMovement` (`Character.CharacterMovement` _enemyattachedto))
            (set `/Game/TopDown/Blueprints/BP_TopDownCharacter.EnemyInCombatWith` (`self.EnemyAttachedTo`) (`self.UserForInteraction`))
            (set `/Game/TopDown/Blueprints/BP_TopDownCharacter.UpgradeFromCombat` self (`self.UserForInteraction`))
            (set `/Game/TopDown/Blueprints/BP_TopDownCharacter.CombatMode` true (`self.UserForInteraction`))
            (set `/Game/TopDown/Blueprints/BP_TopDownCharacter.AmountOfKeysToPress` (- (`/Game/Enemys/BP_EnemyCrabCharacter.Strength` (`self.EnemyAttachedTo`)) (`/Game/TopDown/Blueprints/BP_TopDownCharacter.StrengthStat` (`self.UserForInteraction`))) (`self.UserForInteraction`))
            (`/Game/TopDown/Blueprints/BP_TopDownCharacter.SelectKeyToPress` (`self.UserForInteraction`))
            (`CharacterMovementComponent.DisableMovement` (`Character.CharacterMovement` (`self.UserForInteraction`))))
          (else
            (message `/Game/JoeStuff/Collectibles/CollectibleInterface.Interact` self)))))
    (:`CastFailed`
      (bind _asbp_enemy_crab_character (cast `/Game/Enemys/BP_EnemyCrabCharacter` OtherActor))
      (if (`/Game/Enemys/BP_EnemyCrabCharacter.IsCarryingItem` _asbp_enemy_crab_character)
        _
        (elif (not (!= (`self.EnemyAttachedTo`) null))
          (set `/Game/Enemys/BP_EnemyCrabCharacter.IsCarryingItem` true _asbp_enemy_crab_character)
          (set `self.IsEnemyGrabbed` true)
          (bind _output_get_2 (set `self.EnemyAttachedTo` _asbp_enemy_crab_character))
          (`KismetSystemLibrary.K2_ClearAndInvalidateTimerHandle` (`/Game/Enemys/BP_EnemyCrabCharacter.MoveTowardsItemTimer` (`self.EnemyAttachedTo`)))
          (`/Game/Enemys/BP_EnemyCrabCharacter.RandomMovementState` (`self.EnemyAttachedTo`))
          (`self.K2_AttachToComponent` (`/Game/Enemys/BP_EnemyCrabCharacter.ItemHoldPos` (`self.EnemyAttachedTo`)) "None" "SnapToTarget" "KeepWorld" "KeepWorld" false))))))

(fn `CheckEnemyGrab`
  (if (`self.IsEnemyGrabbed`)
    (`KismetSystemLibrary.PrintString` "Some other enemy has this!")
    (else
      (`self.OnCollect`))))

(fn `UserConstructionScript`)