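; BP_EnemyTest is a test enemy Blueprint that searches the level for a nearest BP_TestItem when play begins.
; BeginPlay loops over every item and keeps the actor and Cube location with the smallest distance, measured against the stored ClosestItemLoc rather than the enemy's own position.
; MoveToLocation and random-offset nodes are left unconnected, so the enemy never moves toward the item.
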(event `self.ReceiveBeginPlay`
  (bind _outactors (`GameplayStatics.GetAllActorsOfClass` "/Game/Enemys/BP_TestItem.BP_TestItem_C"))
  (for _array_element _outactors
    (bind _returnvalue (`SceneComponent.K2_GetComponentLocation` (`/Game/Enemys/BP_TestItem.Cube` _array_element)))
    (bind _returnvalue_2 (`KismetMathLibrary.Vector_Distance` _returnvalue (`self.ClosestItemLoc`)))
    (if (< _returnvalue_2 (`self.DistanceToClosestItem`))
      (set `self.DistanceToClosestItem` _returnvalue_2)
      (set `self.ClosestItemLoc` _returnvalue)
      (set `self.ClosestItem` _array_element))))

(fn `UserConstructionScript`)