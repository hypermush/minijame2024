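; Box-volume spawner that populates an area with crab enemies, speed, strength and progress collectibles, plus seaweed and seashells.
; SpawnItemsAndEnemys, not triggered within this graph, scatters actors at random XY points inside the inset box, with random yaw for non-enemies.
; Crabs spawn as AI with Strength randomized within one of SpawnerLevel; seashells reuse the seaweed count.
; Spawns are tracked for DeleteEnemies and DeleteItems, which also removes environmentals.
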(event `SpawnItemsAndEnemys`
  (bind _seaweedtospawn (`self.SeaweedToSpawn`))
  (`self.SpawnEnemy` (`self.EnemiesToSpawn`) "/Game/Enemys/BP_EnemyCrabCharacter.BP_EnemyCrabCharacter_C")
  (`self.SpawnItem` (`self.SpeedToSpawn`) "/Game/JoeStuff/Collectibles/BP_SpeedCollectible.BP_SpeedCollectible_C")
  (`self.SpawnItem` (`self.StrengthToSpawn`) "/Game/JoeStuff/Collectibles/BP_StrengthCollectible.BP_StrengthCollectible_C")
  (`self.SpawnItem` (`self.ProgressToSpawn`) "/Game/JoeStuff/Collectibles/BP_ProgressCollectible.BP_ProgressCollectible_C")
  (`self.SpawnEnvironmentals` _seaweedtospawn "/Game/JoeStuff/BP_Seaweed.BP_Seaweed_C")
  (`self.SpawnEnvironmentals` _seaweedtospawn "/Game/JoeStuff/BP_Seashell1.BP_Seashell1_C"))

(fn `DeleteEnemies`
  (for _array_element (`self.EnemiesSpawned`)
    (if (`KismetSystemLibrary.IsValid` _array_element)
      (`self.K2_DestroyActor` _array_element))))

(fn `DeleteItems`
  (for _array_element (`self.ItemsSpawned`)
    (if (`KismetSystemLibrary.IsValid` _array_element)
      (`self.K2_DestroyActor` _array_element))))

(fn `SpawnEnemy`
  (params (AmountToSpawn :type Integer) (ActorToSpawn :type "Pawn Class Reference"))
  (bind (_returnvalue_x _returnvalue_y _returnvalue_z) (`KismetMathLibrary.BreakVector` (`SceneComponent.K2_GetComponentLocation` (`self.Box`))))
  (bind (_returnvalue_x_2 _returnvalue_y_2) (`KismetMathLibrary.BreakVector` (`KismetMathLibrary.RandomPointInBoundingBox` (`SceneComponent.K2_GetComponentLocation` (`self.DefaultSceneRoot`)) (- (`BoxComponent.BoxExtent` (`self.Box`)) (20.0 20.0 0.0)))))
  (for _ (range 1 (+ AmountToSpawn 1))
    (bind _returnvalue (`AIBlueprintHelperLibrary.SpawnAIFromClass` (`local.ActorToSpawn`) null (`KismetMathLibrary.MakeVector` _returnvalue_x_2 _returnvalue_y_2 (+ _returnvalue_z 20.0)) (struct) false null))
    (`KismetArrayLibrary.Array_Add` (`self.EnemiesSpawned`) _returnvalue)
    (bind _asbp_enemy_crab_character (cast `/Game/Enemys/BP_EnemyCrabCharacter` _returnvalue))
    (set `/Game/Enemys/BP_EnemyCrabCharacter.Strength` (`KismetMathLibrary.RandomIntegerInRange` (- (`self.SpawnerLevel`) 1) (+ (`self.SpawnerLevel`) 1)) _asbp_enemy_crab_character)))

(fn `SpawnEnvironmentals`
  (params (AmountToSpawn :type Integer) (ActorToSpawn :type "Actor Class Reference"))
  (bind (_returnvalue_x _returnvalue_y _returnvalue_z) (`KismetMathLibrary.BreakVector` (`SceneComponent.K2_GetComponentLocation` (`self.Box`))))
  (bind (_returnvalue_x_2 _returnvalue_y_2) (`KismetMathLibrary.BreakVector` (`KismetMathLibrary.RandomPointInBoundingBox` (`SceneComponent.K2_GetComponentLocation` (`self.DefaultSceneRoot`)) (- (`BoxComponent.BoxExtent` (`self.Box`)) (20.0 20.0 0.0)))))
  (for _ (range 1 (+ AmountToSpawn 1))
    (bind _returnvalue (`|SpawnActorFromClass` (`local.ActorToSpawn`) (`KismetMathLibrary.MakeTransform` (`KismetMathLibrary.MakeVector` _returnvalue_x_2 _returnvalue_y_2 (+ _returnvalue_z 20.0)) (`KismetMathLibrary.MakeRotator` 0.0 0.0 (`KismetMathLibrary.Conv_IntToDouble` (`KismetMathLibrary.RandomIntegerInRange` 0 360)))) "AdjustIfPossibleButAlwaysSpawn" "OverrideRootScale" null null))
    (`KismetArrayLibrary.Array_Add` (`self.ItemsSpawned`) _returnvalue)))

(fn `SpawnItem`
  (params (AmountToSpawn :type Integer) (ActorToSpawn :type "Actor Class Reference"))
  (bind (_returnvalue_x _returnvalue_y _returnvalue_z) (`KismetMathLibrary.BreakVector` (`SceneComponent.K2_GetComponentLocation` (`self.Box`))))
  (bind (_returnvalue_x_2 _returnvalue_y_2) (`KismetMathLibrary.BreakVector` (`KismetMathLibrary.RandomPointInBoundingBox` (`SceneComponent.K2_GetComponentLocation` (`self.DefaultSceneRoot`)) (- (`BoxComponent.BoxExtent` (`self.Box`)) (20.0 20.0 0.0)))))
  (for _ (range 1 (+ AmountToSpawn 1))
    (bind _returnvalue (`|SpawnActorFromClass` (`local.ActorToSpawn`) (`KismetMathLibrary.MakeTransform` (`KismetMathLibrary.MakeVector` _returnvalue_x_2 _returnvalue_y_2 (+ _returnvalue_z 20.0)) (`KismetMathLibrary.MakeRotator` 0.0 0.0 (`KismetMathLibrary.Conv_IntToDouble` (`KismetMathLibrary.RandomIntegerInRange` 0 360)))) "AdjustIfPossibleButAlwaysSpawn" "OverrideRootScale" null null))
    (`KismetArrayLibrary.Array_Add` (`self.ItemsSpawned`) _returnvalue)))

(fn `UserConstructionScript`)