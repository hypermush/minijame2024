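; Enemy crab character that wanders in on a BP_TestItem in progressively more accurate moves.
; FindClosestItem picks the item on BeginPlay, and on Tick while none is set, measuring from the stored item location rather than the crab.
; When stationary, Tick waits, then calls AIMoveTo toward the item with a random offset back toward the crab.
; The offset scales with distance and PercentToMoveTowardsLoc, which steps down to zero with each move.
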(event `self.ReceiveBeginPlay`
  (`self.FindClosestItem`))

(event `self.ReceiveTick`
  (params (DeltaSeconds :type "Float (single-precision)"))
  (bind (_closestitemloc_x _closestitemloc_y) (`KismetMathLibrary.BreakVector` (`self.ClosestItemLoc`)))
  (bind (_returnvalue_x _returnvalue_y _returnvalue_z) (`KismetMathLibrary.BreakVector` (`SceneComponent.K2_GetComponentLocation` (`self.Mesh`))))
  (bind (_returnvalue_x_2 _returnvalue_y_2) (`KismetMathLibrary.BreakVector` (`KismetMathLibrary.GetDirectionUnitVector` (`SceneComponent.K2_GetComponentLocation` (`self.Mesh`)) (`self.ClosestItemLoc`))))
  (bind _returnvalue (* (`KismetMathLibrary.Vector_Distance` (`SceneComponent.K2_GetComponentLocation` (`self.Mesh`)) (`self.ClosestItemLoc`)) (`self.PercentToMoveTowardsLoc`)))
  (bind _returnvalue_2 (`KismetMathLibrary.RandomFloatInRange` 0.0 _returnvalue))
  (bind (_returnvalue_x_3 _returnvalue_y_3) (`KismetMathLibrary.BreakVector` (+ (`KismetMathLibrary.MakeVector` _closestitemloc_x _closestitemloc_y) (`KismetMathLibrary.MakeVector` (* _returnvalue_2 (`self.DirectionToMultiplyX`)) (* (`KismetMathLibrary.RandomFloatInRange` 0.0 _returnvalue) (`self.DirectionToMultiplyY`))))))
  (if (not (!= (`self.ClosestItem`) null))
    (`self.FindClosestItem`))
  (if (== (`KismetMathLibrary.VSize` (`MovementComponent.Velocity` (`self.CharacterMovement`))) 0.0)
    (`KismetSystemLibrary.Delay` 3.0)
    (`KismetSystemLibrary.PrintString` (`KismetStringLibrary.Conv_DoubleToString` _returnvalue_2))
    (if (>= _returnvalue_x_2 0.0)
      (set `self.DirectionToMultiplyX` -1)
      (else
        (set `self.DirectionToMultiplyX` 1)))
    (if (>= _returnvalue_y_2 0.0)
      (set `self.DirectionToMultiplyY` -1)
      (else
        (set `self.DirectionToMultiplyY` 1)))
    (`|AIMoveTo` self (`KismetMathLibrary.MakeVector` _returnvalue_x_3 _returnvalue_y_3 _returnvalue_z) null 5.0 true
      (:`then`
        (if (> 0.0 (+ (`self.PercentToMoveTowardsLoc`) -0.1))
          (set `self.PercentToMoveTowardsLoc` 0.0)
          (else
            (set `self.PercentToMoveTowardsLoc` (+ (`self.PercentToMoveTowardsLoc`) -0.1))))))))

(fn `FindClosestItem`
  (bind _outactors (`GameplayStatics.GetAllActorsOfClass` "/Game/Enemys/BP_TestItem.BP_TestItem_C"))
  (for _array_element _outactors
    (bind _returnvalue (`SceneComponent.K2_GetComponentLocation` (`/Game/Enemys/BP_TestItem.Cube` _array_element)))
    (bind _returnvalue_2 (`KismetMathLibrary.Vector_Distance` _returnvalue (`self.ClosestItemLoc`)))
    (if (< _returnvalue_2 (`self.DistanceToClosestItem`))
      (set `self.DistanceToClosestItem` _returnvalue_2)
      (set `self.ClosestItemLoc` _returnvalue)
      (set `self.ClosestItem` _array_element))))

(fn `UserConstructionScript`)